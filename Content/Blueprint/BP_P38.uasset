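; BP_P38 is a player-controlled P-38 plane pawn that constantly flies forward and can fire rockets.
; Tick spins the left and right propellers and feeds forward movement input to a FloatingPawnMovement component.
; Roll and Pitch axes rotate the actor locally, clamped and scaled by rotation speed and delta time.
; Boost input raises max speed while held, and Fire spawns a BP_Rocket at the Arrow component's transform.
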(event `self.ReceiveTick`
  (params (DeltaSeconds :type "Float (single-precision)"))
  ;[1 1 1] Left Pro
  (`SceneComponent.K2_AddLocalRotation` (`self.Left`) (`KismetMathLibrary.MakeRotator` (* (`self.ProSpeed`) (`GameplayStatics.GetWorldDeltaSeconds`))) false false)
  ;[1 1 1] Right Pro
  (`SceneComponent.K2_AddLocalRotation` (`self.Right`) (`KismetMathLibrary.MakeRotator` (* (`self.ProSpeed`) (`GameplayStatics.GetWorldDeltaSeconds`))) false false)
  ;[1 1 1] Forward
  (`self.AddMovementInput` (`self.GetActorForwardVector`)))

(event `InputAxis|Roll`
  (params (AxisValue :type "Float (single-precision)"))
  ;[1 1 1] Roll
  (`self.K2_AddActorLocalRotation` (`KismetMathLibrary.MakeRotator` (* (`KismetMathLibrary.FClamp` AxisValue -1.0) (`self.RotationSpeed`) (`GameplayStatics.GetWorldDeltaSeconds`)))))

(event `InputAxis|Pitch`
  (params (AxisValue :type "Float (single-precision)"))
  ;[1 1 1] Pitch
  (`self.K2_AddActorLocalRotation` (`KismetMathLibrary.MakeRotator` 0.0 (* (`KismetMathLibrary.FClamp` AxisValue -1.0) (`self.RotationSpeed`) (`GameplayStatics.GetWorldDeltaSeconds`)))))

(event `InputAction|BOost`
  (params (Key :type "Key Structure"))
  ;[1 1 1] Boost
  (:`Pressed`
    (set `FloatingPawnMovement.MaxSpeed` (`self.Boost`) (`self.FloatingPawnMovement`)))
  (:`Released`
    (set `FloatingPawnMovement.MaxSpeed` 1200.0 (`self.FloatingPawnMovement`))))

(event `InputAction|Fire`
  (params (Key :type "Key Structure"))
  (:`Pressed`
    (`|SpawnActorFromClass` "/Game/Blueprint/BP_Rocket.BP_Rocket_C" (`SceneComponent.K2_GetComponentToWorld` (`self.Arrow`)) "Undefined" "OverrideRootScale" null null)))

(fn `UserConstructionScript`)